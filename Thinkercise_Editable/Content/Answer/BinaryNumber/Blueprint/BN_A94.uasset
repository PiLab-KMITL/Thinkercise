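; Answer-set actor from the BinaryNumber folder, with one correct and two wrong answers that the player hits with either hand.
; Tick slides AllAnswer to a relative target and destroys the actor after a delay.
; Overlaps cast to RightHandCheck or LeftHandCheck, call that hand's combo score function, and add or reset the ComboUI combo.
; Each hit also plays a sound, spawns a water-ball effect and destroys the actor.
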(event `self.ReceiveTick`
  (params (DeltaSeconds :type "Float (single-precision)"))
  (`|ExecutionSequence`
    (:`then_0`
      (`KismetSystemLibrary.MoveComponentTo` (`self.AllAnswer`) (-1800.0 0.0 0.0) (struct) false false 3.0))
    (:`then_1`
      (`KismetSystemLibrary.Delay` 4.5)
      (`self.K2_DestroyActor`))))

(event `self.WrongAnswer.OnComponentBeginOverlap`
  (params (OverlappedComponent :type "PrimitiveComponent Object Reference") (OtherActor :type "Actor Object Reference") (OtherComp :type "PrimitiveComponent Object Reference") (OtherBodyIndex :type Integer) (bFromSweep :type Boolean) (SweepResult :type "HitResult Structure (by ref)"))
  ;[1 1 1] Wrong Score System
  (`|ExecutionSequence`
    (:`then_0`
      (bind _asright_hand_check (cast `/Game/HandCheck/RightHandCheck` OtherActor))
      (`GameplayStatics.PlaySound2D` "/Game/Sound/131657__bertrof__game-sound-wrong.131657__bertrof__game-sound-wrong" 1.0 1.0 0.0 null null)
      (`/Game/HandCheck/RightHandCheck.R_ComboScore` _asright_hand_check)
      (bind _outactors (`GameplayStatics.GetAllActorsOfClass` "/Game/UI/bluprint/ComboUI.ComboUI_C"))
      (`/Game/UI/bluprint/ComboUI.ResetCombo` _outactors)
      (`|SpawnActorFromClass` "/Game/FXVarietyPack/Blueprints/BP_ky_waterBallHit.BP_ky_waterBallHit_C" (`SceneComponent.K2_GetComponentToWorld` (`self.WrongAnswer`)) "AlwaysSpawn" "OverrideRootScale" null null)
      (`self.K2_DestroyActor`))
    (:`then_1`
      (bind _asleft_hand_check (cast `/Game/HandCheck/LeftHandCheck` OtherActor))
      (`GameplayStatics.PlaySound2D` "/Game/Sound/131657__bertrof__game-sound-wrong.131657__bertrof__game-sound-wrong" 1.0 1.0 0.0 null null)
      (`/Game/HandCheck/LeftHandCheck.L_ComboScore` _asleft_hand_check)
      (bind _outactors_2 (`GameplayStatics.GetAllActorsOfClass` "/Game/UI/bluprint/ComboUI.ComboUI_C"))
      (`/Game/UI/bluprint/ComboUI.ResetCombo` _outactors_2)
      (`|SpawnActorFromClass` "/Game/FXVarietyPack/Blueprints/BP_ky_waterBallHit.BP_ky_waterBallHit_C" (`SceneComponent.K2_GetComponentToWorld` (`self.WrongAnswer`)) "AlwaysSpawn" "OverrideRootScale" null null)
      (`self.K2_DestroyActor`))))

(event `self.CorrectAnswer.OnComponentBeginOverlap`
  (params (OverlappedComponent :type "PrimitiveComponent Object Reference") (OtherActor :type "Actor Object Reference") (OtherComp :type "PrimitiveComponent Object Reference") (OtherBodyIndex :type Integer) (bFromSweep :type Boolean) (SweepResult :type "HitResult Structure (by ref)"))
  ;[1 1 1] Correct Score System
  (`|ExecutionSequence`
    (:`then_0`
      (bind _asright_hand_check (cast `/Game/HandCheck/RightHandCheck` OtherActor))
      (`GameplayStatics.PlaySound2D` "/Game/Sound/131660__bertrof__game-sound-correct.131660__bertrof__game-sound-correct" 1.0 1.0 0.0 null null)
      (`/Game/HandCheck/RightHandCheck.R_ComboScore` _asright_hand_check)
      (bind _outactors (`GameplayStatics.GetAllActorsOfClass` "/Game/UI/bluprint/ComboUI.ComboUI_C"))
      (`/Game/UI/bluprint/ComboUI.Add Combo` _outactors)
      (`|SpawnActorFromClass` "/Game/FXVarietyPack/Blueprints/BP_ky_waterBallHit.BP_ky_waterBallHit_C" (`SceneComponent.K2_GetComponentToWorld` (`self.CorrectAnswer`)) "AlwaysSpawn" "OverrideRootScale" null null)
      (`self.K2_DestroyActor`))
    (:`then_1`
      (bind _asleft_hand_check (cast `/Game/HandCheck/LeftHandCheck` OtherActor))
      (`GameplayStatics.PlaySound2D` "/Game/Sound/131660__bertrof__game-sound-correct.131660__bertrof__game-sound-correct" 1.0 1.0 0.0 null null)
      (`/Game/HandCheck/LeftHandCheck.L_ComboScore` _asleft_hand_check)
      (bind _outactors_2 (`GameplayStatics.GetAllActorsOfClass` "/Game/UI/bluprint/ComboUI.ComboUI_C"))
      (`/Game/UI/bluprint/ComboUI.Add Combo` _outactors_2)
      (`|SpawnActorFromClass` "/Game/FXVarietyPack/Blueprints/BP_ky_waterBallHit.BP_ky_waterBallHit_C" (`SceneComponent.K2_GetComponentToWorld` (`self.CorrectAnswer`)) "AlwaysSpawn" "OverrideRootScale" null null)
      (`self.K2_DestroyActor`))))

(event `self.WrongAnswer1.OnComponentBeginOverlap`
  (params (OverlappedComponent :type "PrimitiveComponent Object Reference") (OtherActor :type "Actor Object Reference") (OtherComp :type "PrimitiveComponent Object Reference") (OtherBodyIndex :type Integer) (bFromSweep :type Boolean) (SweepResult :type "HitResult Structure (by ref)"))
  ;[1 1 1] Wrong2 Score System
  (`|ExecutionSequence`
    (:`then_0`
      (bind _asright_hand_check (cast `/Game/HandCheck/RightHandCheck` OtherActor))
      (`GameplayStatics.PlaySound2D` "/Game/Sound/131657__bertrof__game-sound-wrong.131657__bertrof__game-sound-wrong" 1.0 1.0 0.0 null null)
      (`/Game/HandCheck/RightHandCheck.R_ComboScore` _asright_hand_check)
      (bind _outactors (`GameplayStatics.GetAllActorsOfClass` "/Game/UI/bluprint/ComboUI.ComboUI_C"))
      (`/Game/UI/bluprint/ComboUI.ResetCombo` _outactors)
      (`|SpawnActorFromClass` "/Game/FXVarietyPack/Blueprints/BP_ky_waterBallHit.BP_ky_waterBallHit_C" (`SceneComponent.K2_GetComponentToWorld` (`self.WrongAnswer1`)) "AlwaysSpawn" "OverrideRootScale" null null)
      (`self.K2_DestroyActor`))
    (:`then_1`
      (bind _asleft_hand_check (cast `/Game/HandCheck/LeftHandCheck` OtherActor))
      (`GameplayStatics.PlaySound2D` "/Game/Sound/131657__bertrof__game-sound-wrong.131657__bertrof__game-sound-wrong" 1.0 1.0 0.0 null null)
      (`/Game/HandCheck/LeftHandCheck.L_ComboScore` _asleft_hand_check)
      (bind _outactors_2 (`GameplayStatics.GetAllActorsOfClass` "/Game/UI/bluprint/ComboUI.ComboUI_C"))
      (`/Game/UI/bluprint/ComboUI.ResetCombo` _outactors_2)
      (`|SpawnActorFromClass` "/Game/FXVarietyPack/Blueprints/BP_ky_waterBallHit.BP_ky_waterBallHit_C" (`SceneComponent.K2_GetComponentToWorld` (`self.WrongAnswer1`)) "AlwaysSpawn" "OverrideRootScale" null null)
      (`self.K2_DestroyActor`))))

(fn `UserConstructionScript`)